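; BP_Kyoko is a 2D sprite Blueprint for Kyoko that switches flipbook animations on spawn and when damaged.
; SetFlipBook looks up a flipbook by name in the FlipBooks map, applies it and returns its total duration.
; BeginPlay plays "Start" and AnyDamage plays "Dab", each feeding that duration into a Retriggerable Delay before switching to "Idle".
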(event Game|Damage|EventAnyDamage
  (params (Damage :type Float%20%28single-precision%29) (DamageType :type Damage%20Type%20Object%20Reference) (InstigatedBy :type Controller%20Object%20Reference) (DamageCauser :type Actor%20Object%20Reference))
  (bind _returnvalue (CallFunction|SetFlipBook "Dab"))
  (Utilities|FlowControl|RetriggerableDelay _returnvalue)
  (CallFunction|SetFlipBook "Idle"))

(event EventBeginPlay
  (bind _returnvalue (CallFunction|SetFlipBook "Start"))
  (Utilities|FlowControl|RetriggerableDelay _returnvalue)
  (CallFunction|SetFlipBook "Idle"))

(fn ConstructionScript)

(fn SetFlipBook
  (params (InName :type Name))
  (bind _flipbooks (Variables|Default|GetFlipBooks))
  (bind _value (Utilities|Map|Find _flipbooks InName))
  (Sprite|SetFlipbook (Variables|Default|GetPaperFlipbook) _value)
  (return (Class|PaperFlipbook|GetTotalDuration _value)))